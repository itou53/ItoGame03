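; Main game mode that, on BeginPlay, sets up the on-screen UI and triggers an attack on the player character class.
; A Sequence creates the W_Text widget, adds it to the viewport, then calls StartAttack on the first BP_ThirdPersonCharacter found.
; Its last branch runs a loop with a Delay to add W_Entry_A to the widget's ListView, then prints the list items' display names.
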(event `self.ReceiveBeginPlay`
  (bind _listview_1 (`/Game/UI/W_Text.ListView_1` (`self.W_Main`)))
  (`|ExecutionSequence`
    (:`then_0`
      (bind _returnvalue (`|CreateWidget` "/Game/UI/W_Text.W_Text_C"))
      (bind _output_get (set `self.W_Main` _returnvalue))
      (`UserWidget.AddToViewport` _output_get 0))
    (:`then_1`
      (bind _outactors (`GameplayStatics.GetAllActorsOfClass` "/Game/ThirdPerson/Blueprints/BP_ThirdPersonCharacter.BP_ThirdPersonCharacter_C"))
      (`/Game/ThirdPerson/Blueprints/BP_ThirdPersonCharacter.StartAttack` (`|GetArrayItem` _outactors)))
    (:`then_2`
      (for _ (range 6)
        (`KismetSystemLibrary.Delay` 1.0)
        (`ListView.AddItem` _listview_1 "/Game/UI/W_Entry_A.W_Entry_A"))
      (for _array_element (`ListView.GetListItems` _listview_1)
        (`KismetSystemLibrary.PrintString` (`KismetSystemLibrary.GetDisplayName` _array_element))))))

(fn `UserConstructionScript`)